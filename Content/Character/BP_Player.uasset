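; BP_Player is the player character Blueprint, handling basic movement, camera look and jumping through Enhanced Input.
; On BeginPlay it adds the Player_IMC mapping context to the controlling player's local input subsystem.
; Look_IA drives controller yaw and pitch, Movement_IA moves along the actor's right and forward vectors, and Jump_IA triggers a jump.
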(event Input|EnhancedActionEvents|EnhancedInputActionMovement_IA
  (params (ActionValue :type Vector%202D%20Structure) (ElapsedSeconds :type Float%20%28double-precision%29) (TriggeredSeconds :type Float%20%28double-precision%29) (InputAction :type Input%20Action%20Object%20Reference :default "/Game/Character/Movement/Movement_IA.Movement_IA"))
  ;[0.15 0.15 0.15 0.5] Movement
  (:Triggered
    (Pawn|Input|AddMovementInput (Transformation|GetActorRightVector) (.x ActionValue) false)
    (Pawn|Input|AddMovementInput (Transformation|GetActorForwardVector) (.y ActionValue) false)))

(event Input|EnhancedActionEvents|EnhancedInputActionLook_IA
  (params (ActionValue :type Vector%202D%20Structure) (ElapsedSeconds :type Float%20%28double-precision%29) (TriggeredSeconds :type Float%20%28double-precision%29) (InputAction :type Input%20Action%20Object%20Reference :default "/Game/Character/Movement/Look_IA.Look_IA"))
  ;[0.15 0.15 0.15 0.5] Camera Control
  (:Triggered
    (Pawn|Input|AddControllerYawInput (.x ActionValue))
    (Pawn|Input|AddControllerPitchInput (.y ActionValue))))

(event Input|EnhancedActionEvents|EnhancedInputActionJump_IA
  (params (ActionValue :type Boolean) (ElapsedSeconds :type Float%20%28double-precision%29) (TriggeredSeconds :type Float%20%28double-precision%29) (InputAction :type Input%20Action%20Object%20Reference :default "/Game/Character/Movement/Jump_IA.Jump_IA"))
  (Character|Jump))

(event EventBeginPlay
  ;[0.15 0.15 0.15 0.5] Input Controls
  (bind _asplayer_controller (Utilities|Casting|CastToPlayerController (Pawn|GetController)))
  (Utilities|IsValid (PlayerController|LocalPlayerSubsystems|GetEnhancedInputLocalPlayerSubsystem _asplayer_controller)
    (:Is%20Valid
      (Input|AddMappingContext (PlayerController|LocalPlayerSubsystems|GetEnhancedInputLocalPlayerSubsystem _asplayer_controller) "/Game/Character/Movement/Player_IMC.Player_IMC" 0 "(bIgnoreAllPressedKeysUntilRelease=True,bForceImmediately=False,bNotifyUserSettings=False)"))))

(fn ConstructionScript)